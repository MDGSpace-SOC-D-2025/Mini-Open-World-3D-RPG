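; BP_Hero is the hero character Blueprint, handling a speed-based dash and the player's on-screen HUD.
; The Dash input raises CharacterMovement's max walk speed sharply while triggered and sets it to a fixed normal speed on completion.
; BeginPlay adds health and stamina widgets to the viewport, and HealthComp updates refresh the health bar through the stored HUD reference.
; The stamina widget receives no data here, and dashing has no stamina check.
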(event OnHealthUpdate(HealthComp)
  (bind _hud (Variables|Default|GetHUD))
  (Utilities|IsValid _hud
    (:Is%20Valid
      (Default|SetHP (Variables|/Game/Hero/UI/WB_HP.WB_HP_C|GetWB_HealthBar _hud) (Variables|Default|GetHealthComp)))))

(event Input|EnhancedActionEvents|EnhancedInputActionDash
  (params (ActionValue :type Vector%202D%20Structure) (ElapsedSeconds :type Float%20%28double-precision%29) (TriggeredSeconds :type Float%20%28double-precision%29) (InputAction :type Input%20Action%20Object%20Reference :default "/Game/Hero/MyInput/Actions/Dash.Dash"))
  (bind _charactermovement (Variables|Character|GetCharacterMovement))
  (:Triggered
    (Variables|/Script/Engine.CharacterMovementComponent|SetMaxWalkSpeed _charactermovement 5e+03))
  (:Completed
    (Variables|/Script/Engine.CharacterMovementComponent|SetMaxWalkSpeed _charactermovement 6e+02)))

(event EventBeginPlay
  (Utilities|FlowControl|Sequence
    (:then_0
      (bind _returnvalue (UserInterface|CreateWidget "/Game/Hero/UI/WB_HP.WB_HP_C"))
      (bind _output_get (Variables|Default|SetHUD _returnvalue))
      (UserInterface|Viewport|AddtoViewport _output_get 0)
      (Default|SetHP (Variables|/Game/Hero/UI/WB_HP.WB_HP_C|GetWB_HealthBar _output_get) (Variables|Default|GetHealthComp)))
    (:then_1
      (bind _returnvalue_2 (UserInterface|CreateWidget "/Game/Hero/UI/WB_Stamina.WB_Stamina_C"))
      (UserInterface|Viewport|AddtoViewport _returnvalue_2 0))))

(fn ConstructionScript)